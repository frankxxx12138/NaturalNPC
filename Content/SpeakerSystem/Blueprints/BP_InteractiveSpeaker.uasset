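; Interactive VR speaker actor with buttons that play Jazz, Dance or Blues music and a Pause toggle.
; Overlaps from components tagged MusicButtonFinger track the hovered button by name, and left or right grab input activates it; OnClicked events also trigger the same presses.
; Choosing a track stops the current audio, clears pause, swaps the sound and fades it in briefly.
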(event `PressJazzButton`
  (`self.PlaySelectedMusic` (`self.JazzMusic`)))

(event `self.Button_Jazz.OnClicked`
  (params (TouchedComponent :type "PrimitiveComponent Object Reference") (ButtonPressed :type "Key Structure"))
  (`self.PressJazzButton`))

(event `PressPauseButton`
  (bind _speakeraudio (`self.SpeakerAudio`))
  (if (`self.IsPaused`)
    (`AudioComponent.SetPaused` _speakeraudio false)
    (set `self.IsPaused` false)
    (else
      (`AudioComponent.SetPaused` _speakeraudio true)
      (set `self.IsPaused` true))))

(event `PressDanceButton`
  (`self.PlaySelectedMusic` (`self.DanceMusic`)))

(event `self.Button_Blues.OnClicked`
  (params (TouchedComponent :type "PrimitiveComponent Object Reference") (ButtonPressed :type "Key Structure"))
  (`self.PressBluesButton`))

(event `self.ReceiveBeginPlay`
  (`self.EnableInput` (`GameplayStatics.GetPlayerController` 0)))

(event `self.Button_Dance.OnClicked`
  (params (TouchedComponent :type "PrimitiveComponent Object Reference") (ButtonPressed :type "Key Structure"))
  (`self.PressDanceButton`))

(event `PressBluesButton`
  (`self.PlaySelectedMusic` (`self.BluesMusic`)))

(event `self.Button_Pause.OnClicked`
  (params (TouchedComponent :type "PrimitiveComponent Object Reference") (ButtonPressed :type "Key Structure"))
  (`self.PressPauseButton`))

(event `EnhancedInput|/Game/XRFramework/Input/Actions/IA_Grab_Right_Pressed`
  (params (ActionValue :type "Float (double-precision)") (ElapsedSeconds :type "Float (double-precision)") (TriggeredSeconds :type "Float (double-precision)") (InputAction :type "InputAction Object Reference" :default "/Game/XRFramework/Input/Actions/IA_Grab_Right_Pressed.IA_Grab_Right_Pressed"))
  (:`Started`
    (`self.TryActivateHoveredMusicButton`)))

(event `EnhancedInput|/Game/XRFramework/Input/Actions/IA_Grab_Left_Pressed`
  (params (ActionValue :type "Float (double-precision)") (ElapsedSeconds :type "Float (double-precision)") (TriggeredSeconds :type "Float (double-precision)") (InputAction :type "InputAction Object Reference" :default "/Game/XRFramework/Input/Actions/IA_Grab_Left_Pressed.IA_Grab_Left_Pressed"))
  (:`Started`
    (`self.TryActivateHoveredMusicButton`)))

(event `self.Button_Jazz.OnComponentBeginOverlap`
  (params (OverlappedComponent :type "PrimitiveComponent Object Reference") (OtherActor :type "Actor Object Reference") (OtherComp :type "PrimitiveComponent Object Reference") (OtherBodyIndex :type Integer) (bFromSweep :type Boolean) (SweepResult :type "HitResult Structure (by ref)"))
  (if (`ActorComponent.ComponentHasTag` OtherComp "MusicButtonFinger")
    (set `self.HoveredMusicButton` "Jazz")))

(event `self.Button_Dance.OnComponentBeginOverlap`
  (params (OverlappedComponent :type "PrimitiveComponent Object Reference") (OtherActor :type "Actor Object Reference") (OtherComp :type "PrimitiveComponent Object Reference") (OtherBodyIndex :type Integer) (bFromSweep :type Boolean) (SweepResult :type "HitResult Structure (by ref)"))
  (if (`ActorComponent.ComponentHasTag` OtherComp "MusicButtonFinger")
    (set `self.HoveredMusicButton` "Dance")))

(event `self.Button_Blues.OnComponentBeginOverlap`
  (params (OverlappedComponent :type "PrimitiveComponent Object Reference") (OtherActor :type "Actor Object Reference") (OtherComp :type "PrimitiveComponent Object Reference") (OtherBodyIndex :type Integer) (bFromSweep :type Boolean) (SweepResult :type "HitResult Structure (by ref)"))
  (if (`ActorComponent.ComponentHasTag` OtherComp "MusicButtonFinger")
    (set `self.HoveredMusicButton` "Blues")))

(event `self.Button_Pause.OnComponentBeginOverlap`
  (params (OverlappedComponent :type "PrimitiveComponent Object Reference") (OtherActor :type "Actor Object Reference") (OtherComp :type "PrimitiveComponent Object Reference") (OtherBodyIndex :type Integer) (bFromSweep :type Boolean) (SweepResult :type "HitResult Structure (by ref)"))
  (if (`ActorComponent.ComponentHasTag` OtherComp "MusicButtonFinger")
    (set `self.HoveredMusicButton` "Pause")))

(event `self.Button_Jazz.OnComponentEndOverlap`
  (params (OverlappedComponent :type "PrimitiveComponent Object Reference") (OtherActor :type "Actor Object Reference") (OtherComp :type "PrimitiveComponent Object Reference") (OtherBodyIndex :type Integer))
  (if (`ActorComponent.ComponentHasTag` OtherComp "MusicButtonFinger")
    (set `self.HoveredMusicButton` "None")))

(event `self.Button_Dance.OnComponentEndOverlap`
  (params (OverlappedComponent :type "PrimitiveComponent Object Reference") (OtherActor :type "Actor Object Reference") (OtherComp :type "PrimitiveComponent Object Reference") (OtherBodyIndex :type Integer))
  (if (`ActorComponent.ComponentHasTag` OtherComp "MusicButtonFinger")
    (set `self.HoveredMusicButton` "None")))

(event `self.Button_Blues.OnComponentEndOverlap`
  (params (OverlappedComponent :type "PrimitiveComponent Object Reference") (OtherActor :type "Actor Object Reference") (OtherComp :type "PrimitiveComponent Object Reference") (OtherBodyIndex :type Integer))
  (if (`ActorComponent.ComponentHasTag` OtherComp "MusicButtonFinger")
    (set `self.HoveredMusicButton` "None")))

(event `self.Button_Pause.OnComponentEndOverlap`
  (params (OverlappedComponent :type "PrimitiveComponent Object Reference") (OtherActor :type "Actor Object Reference") (OtherComp :type "PrimitiveComponent Object Reference") (OtherBodyIndex :type Integer))
  (if (`ActorComponent.ComponentHasTag` OtherComp "MusicButtonFinger")
    (set `self.HoveredMusicButton` "None")))

(fn `PlaySelectedMusic`
  (params (NewMusic :type "SoundBase Object Reference"))
  (bind _speakeraudio (`self.SpeakerAudio`))
  (bind _speakeraudio_2 (`self.SpeakerAudio`))
  (`AudioComponent.Stop` _speakeraudio)
  (`AudioComponent.SetPaused` _speakeraudio false)
  (set `self.IsPaused` false)
  (`AudioComponent.SetSound` _speakeraudio_2 NewMusic)
  (`AudioComponent.FadeIn` _speakeraudio_2 0.25 1.0 0.0 "Linear"))

(fn `TryActivateHoveredMusicButton`
  (switch `name` (`self.HoveredMusicButton`)
    (:`Jazz`
      (`self.PressJazzButton`))
    (:`Dance`
      (`self.PressDanceButton`))
    (:`Blues`
      (`self.PressBluesButton`))
    (:`Pause`
      (`self.PressPauseButton`))))

(fn `UserConstructionScript`)